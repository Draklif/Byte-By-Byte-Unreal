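; FL_Utilities is a Blueprint function library with helpers for random item lookup and notification popups.
; GetRandomItem picks a random DT_Items row by turning an integer between one and the row count into a row name, so it relies on numerically named rows.
; PlayTip creates a WBP_NotificationPopup with the given title, description and delay, then adds it to the viewport.
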(fn `GetRandomItem`
  (returns (Found :type Boolean) (Row :type "/Game/Blueprints/Structs/S_Item Structure"))
  (bind _outrownames (`DataTableFunctionLibrary.GetDataTableRowNames` "/Game/Blueprints/Tables/DT_Items.DT_Items"))
  (bind _returnvalue (`|GetDataTableRow` "/Game/Blueprints/Tables/DT_Items.DT_Items" (`KismetStringLibrary.Conv_StringToName` (`KismetStringLibrary.Conv_IntToString` (`KismetMathLibrary.RandomIntegerInRange` 1 (`KismetArrayLibrary.Array_Length` _outrownames)))))
    (:`then`
      (return true _returnvalue))
    (:`RowNotFound`
      (return false))))

(fn `PlayTip`
  (params (`Title Text` :type Text) (`Description Text` :type Text) (Delay :type "Float (single-precision)"))
  (bind _returnvalue (`|CreateWidget` "/Game/Blueprints/UI/WBP_NotificationPopup.WBP_NotificationPopup_C" null `Title Text` `Description Text` Delay))
  (`UserWidget.AddToViewport` _returnvalue 0))