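; Blueprint function library that gives global access to the game's BP_GameInstance and the key objects it references.
; GetGameInstance casts the current game instance to BP_GameInstance, and every other getter builds on it.
; Getters for the world, shop, activity and stage managers and the player each validity-check the stored reference and return it with an IsValid flag.
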(fn `GetActivityManager`
  (returns (IsValid :type Boolean) (ActivityManager :type "/Game/Blueprints/Managers/BP_ActivityManager Object Reference"))
  (bind _asbp_game_instance (`self.GetGameInstance` null))
  (bind _gi_activitymanager (`/Game/Blueprints/BP_GameInstance.GI_ActivityManager` _asbp_game_instance))
  (`/Engine/EditorBlueprintResources/StandardMacros.IsValid` _gi_activitymanager
    (:`Is Valid`
      (return true _gi_activitymanager))
    (:`Is Not Valid`
      (return false null))))

(fn `GetGameInstance`
  (returns (`AsBP Game Instance` :type "/Game/Blueprints/BP_GameInstance Object Reference"))
  (bind _asbp_game_instance (cast `/Game/Blueprints/BP_GameInstance` (`GameplayStatics.GetGameInstance` null)))
  (return _asbp_game_instance))

(fn `GetPlayer`
  (returns (IsValid :type Boolean) (Player :type "/Game/Blueprints/Managers/BP_Player Object Reference"))
  (bind _asbp_game_instance (`self.GetGameInstance` null))
  (bind _gi_player (`/Game/Blueprints/BP_GameInstance.GI_Player` _asbp_game_instance))
  (`/Engine/EditorBlueprintResources/StandardMacros.IsValid` _gi_player
    (:`Is Valid`
      (return true _gi_player))
    (:`Is Not Valid`
      (return false null))))

(fn `GetShopManager`
  (returns (IsValid :type Boolean) (ShopManager :type "/Game/Blueprints/Managers/BP_ShopManager Object Reference"))
  (bind _asbp_game_instance (`self.GetGameInstance` null))
  (bind _gi_shopmanager (`/Game/Blueprints/BP_GameInstance.GI_ShopManager` _asbp_game_instance))
  (`/Engine/EditorBlueprintResources/StandardMacros.IsValid` _gi_shopmanager
    (:`Is Valid`
      (return true _gi_shopmanager))
    (:`Is Not Valid`
      (return false null))))

(fn `GetStageManager`
  (returns (IsValid :type Boolean) (StageManager :type "/Game/Blueprints/Managers/BP_StageManager Object Reference"))
  (bind _asbp_game_instance (`self.GetGameInstance` null))
  (bind _gi_stagemanager (`/Game/Blueprints/BP_GameInstance.GI_StageManager` _asbp_game_instance))
  (`/Engine/EditorBlueprintResources/StandardMacros.IsValid` _gi_stagemanager
    (:`Is Valid`
      (return true _gi_stagemanager))
    (:`Is Not Valid`
      (return false _gi_stagemanager))))

(fn `GetWorldManager`
  (returns (IsValid :type Boolean) (WorldManager :type "/Game/Blueprints/Managers/BP_WorldManager Object Reference"))
  (bind _asbp_game_instance (`self.GetGameInstance` null))
  (bind _gi_worldmanager (`/Game/Blueprints/BP_GameInstance.GI_WorldManager` _asbp_game_instance))
  (`/Engine/EditorBlueprintResources/StandardMacros.IsValid` _gi_worldmanager
    (:`Is Valid`
      (return true _gi_worldmanager))
    (:`Is Not Valid`
      (return false null))))