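; Manager that runs timed player activities, enforcing per-activity use limits that reset each new day.
; It saves the current activity, start date and usages in the GameInstance, resuming or completing the timer on BeginPlay.
; Completion grants stats, skipping or switching grants halved rewards, and special IDs route work and study through Player and StageManager.
; Helper functions list DT_Activities rows by category and filter them by weekday and time of day.
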(event `self.ReceiveBeginPlay`
  (bind _asbp_game_instance (`/Game/Blueprints/FunctionLibraries/FL_GameInstance.GetGameInstance`))
  (set `self.ActivityUsages` (`/Game/Blueprints/BP_GameInstance.GI_ActivityUsages` _asbp_game_instance))
  (bind (_isvalid _worldmanager) (`/Game/Blueprints/FunctionLibraries/FL_GameInstance.GetWorldManager`))
  (add `/Game/Blueprints/Managers/BP_WorldManager.OnNewDay` _worldmanager (delegate `Reset Activity Usages`))
  (`self.LoadCurrentActivity`))

(event `Reset Activity Usages`
  (`BlueprintMapLibrary.Map_Clear` (`self.ActivityUsages`))
  (bind _asbp_game_instance (`/Game/Blueprints/FunctionLibraries/FL_GameInstance.GetGameInstance`))
  (set `/Game/Blueprints/BP_GameInstance.GI_ActivityUsages` (`self.ActivityUsages`) _asbp_game_instance))

(fn `Execute Activity`
  (params (Activity :type "/Game/Blueprints/Structs/S_Activity Structure (by ref)"))
  (bind (_id _name _uses) (break `/Game/Blueprints/Structs/S_Activity` Activity))
  (bind _activityusages (`self.ActivityUsages`))
  (if (and (`BlueprintMapLibrary.Map_Contains` _activityusages _id) (>= (`BlueprintMapLibrary.Map_Find` _activityusages _id) _uses) (!= _uses -1))
    (`/Game/Blueprints/FunctionLibraries/FL_Utilities.PlayTip` "No more uses" "No more uses remaining for this activity today." 3.0)
    (else
      (if (`KismetSystemLibrary.K2_IsValidTimerHandle` (`self.ActivityTimer`))
        (`/Game/Blueprints/FunctionLibraries/FL_Utilities.PlayTip` "Already on an activity" "You are already in an activity. Skipping." 5.0)
        (`self.Skip Activity`))
      (set `self.ActivityCurrent` Activity)
      (`self.Start Activity` Activity))))

(fn `Filter Activities By Day`
  (params (ActivitiesToFilter :type "Array of /Game/Blueprints/Structs/S_Activity Structure"))
  (returns (Activities :type "Array of /Game/Blueprints/Structs/S_Activity Structure"))
  (locals (FilteredActivities :type "Array of /Game/Blueprints/Structs/S_Activity Structure"))
  (for _array_element ActivitiesToFilter
    (for _array_element_2 (`.AvailableDays_43_28E559CB4D30FDEE9ECC86BC5E31940C` (break `/Game/Blueprints/Structs/S_Activity` _array_element))
      (bind (_isvalid _worldmanager) (`/Game/Blueprints/FunctionLibraries/FL_GameInstance.GetWorldManager`))
      (if _isvalid
        (if (`|EnumEquality` _array_element_2 (`/Game/Blueprints/Managers/BP_WorldManager.DayOfWeek` _worldmanager))
          (`KismetArrayLibrary.Array_AddUnique` (`local.FilteredActivities`) _array_element)
          (break)))))
  (return (`local.FilteredActivities`)))

(fn `Filter Activities By Time of Day`
  (params (ActivitiesToFilter :type "Array of /Game/Blueprints/Structs/S_Activity Structure"))
  (returns (Activities :type "Array of /Game/Blueprints/Structs/S_Activity Structure"))
  (locals (FilteredActivities :type "Array of /Game/Blueprints/Structs/S_Activity Structure"))
  (for _array_element ActivitiesToFilter
    (for _array_element_2 (`.AvailableTime_40_167C65A940D48DA5A16C38B36BE38ED8` (break `/Game/Blueprints/Structs/S_Activity` _array_element))
      (bind (_isvalid _worldmanager) (`/Game/Blueprints/FunctionLibraries/FL_GameInstance.GetWorldManager`))
      (if _isvalid
        (if (`|EnumEquality` _array_element_2 (`/Game/Blueprints/Managers/BP_WorldManager.TimeOfDay` _worldmanager))
          (`KismetArrayLibrary.Array_AddUnique` (`local.FilteredActivities`) _array_element)
          (break)))))
  (return (`local.FilteredActivities`)))

(fn `Get Activities By Category`
  (params (Category :type "/Game/Blueprints/Enums/E_ActivityCategory Enum" :default "NewEnumerator0"))
  (returns (Activities :type "Array of /Game/Blueprints/Structs/S_Activity Structure"))
  (locals (ActivitiesList :type "Array of /Game/Blueprints/Structs/S_Activity Structure"))
  (bind _outrownames (`DataTableFunctionLibrary.GetDataTableRowNames` "/Game/Blueprints/Tables/DT_Activities.DT_Activities"))
  (for _array_element _outrownames
    (bind _returnvalue (`|GetDataTableRow` "/Game/Blueprints/Tables/DT_Activities.DT_Activities" _array_element)
      (:`then`
        (bind (_id _name _uses _stats _availabletime _availabledays _timetocomplete _activitytype _activitycategory) (break `/Game/Blueprints/Structs/S_Activity` _returnvalue))
        (if (and (`|EnumEquality` _activitycategory Category) (`|EnumInequality` _activitytype "NewEnumerator1"))
          (`KismetArrayLibrary.Array_Add` (`local.ActivitiesList`) _returnvalue)))))
  (return (`local.ActivitiesList`)))

(fn `HandleActivityReward`
  (params (Activity :type "/Game/Blueprints/Structs/S_Activity Structure") (Halved :type Boolean))
  (bind (_id _name _uses _stats _availabletime _availabledays _timetocomplete _activitytype) (break `/Game/Blueprints/Structs/S_Activity` Activity))
  (switch `/Game/Blueprints/Enums/E_ActivityType` _activitytype
    (:`NewEnumerator0`
      (bind (_isvalid _player) (`/Game/Blueprints/FunctionLibraries/FL_GameInstance.GetPlayer`))
      (if _isvalid
        (`/Game/Blueprints/Managers/BP_Player.ModifyPlayerStats` _player _stats Halved)
        (`self.OnActivityCompleted`)))
    (:`NewEnumerator1`
      (`self.HandleSpecialActivityReward` (`local.Activity`) Halved))))

(fn `HandleSpecialActivityReward`
  (params (Activity :type "/Game/Blueprints/Structs/S_Activity Structure") (Halved :type Boolean))
  (bind _id (break `/Game/Blueprints/Structs/S_Activity` Activity))
  (bind _halved (`local.Halved`))
  (bind (_isvalid _player) (`/Game/Blueprints/FunctionLibraries/FL_GameInstance.GetPlayer`))
  (if _isvalid
    (switch `int` _id
      (:`200`
        (`/Game/Blueprints/Managers/BP_Player.ModifyMoneyWork` _player _halved)
        (`self.OnActivityCompleted` :!label _label))
      (:`201`
        (`/Game/Blueprints/Managers/BP_Player.ModifyKnowledgeStudy` _player (`BlueprintMapLibrary.Map_Find` (`self.ActivityUsages`) _id) _halved)
        (goto _label))
      (:`202`
        (bind (_isvalid_2 _stagemanager) (`/Game/Blueprints/FunctionLibraries/FL_GameInstance.GetStageManager`))
        (if _isvalid_2
          (`/Game/Blueprints/Managers/BP_StageManager.GoStudy` _stagemanager)
          (goto _label)))
      (:`203`
        (bind (_isvalid_3 _stagemanager_2) (`/Game/Blueprints/FunctionLibraries/FL_GameInstance.GetStageManager`))
        (if _isvalid_3
          (`/Game/Blueprints/Managers/BP_StageManager.GoWork` _stagemanager_2)
          (goto _label))))
    (else
      (goto _label))))

(fn `LoadCurrentActivity`
  (bind _asbp_game_instance (`/Game/Blueprints/FunctionLibraries/FL_GameInstance.GetGameInstance`))
  (bind _gi_activitycurrent (`/Game/Blueprints/BP_GameInstance.GI_ActivityCurrent` _asbp_game_instance))
  (set `self.ActivityCurrent` _gi_activitycurrent)
  (bind (_id _name _uses _stats _availabletime _availabledays _timetocomplete) (break `/Game/Blueprints/Structs/S_Activity` _gi_activitycurrent))
  (if (> _id 0)
    (bind _gi_activitystartdate (`/Game/Blueprints/BP_GameInstance.GI_ActivityStartDate` _asbp_game_instance))
    (if (<= (`KismetMathLibrary.BreakDateTime` _gi_activitystartdate) 1)
      (bind _returnvalue (- _timetocomplete (`KismetMathLibrary.GetTotalSeconds` (- (`/Game/Blueprints/Managers/BP_WorldManager.DateNow` (stale _worldmanager)) _gi_activitystartdate))))
      (bind _returnvalue_2 (`KismetSystemLibrary.K2_SetTimerDelegate` (`|CreateDelegate` :!event `OnFinishActivityTimer`) _returnvalue :!label _label))
      (set `self.ActivityTimer` _returnvalue_2)
      (`self.OnActivityStarted`)
      (else
        (bind (_isvalid _worldmanager) (`/Game/Blueprints/FunctionLibraries/FL_GameInstance.GetWorldManager`))
        (if _isvalid
          (if (<= _returnvalue 0.0)
            (`self.OnFinishActivityTimer`)
            (else
              (goto _label))))))))

(fn `OnFinishActivityTimer`
  (bind _asbp_game_instance (`/Game/Blueprints/FunctionLibraries/FL_GameInstance.GetGameInstance`))
  (set `/Game/Blueprints/BP_GameInstance.GI_ActivityCurrent` (struct) _asbp_game_instance)
  (set `/Game/Blueprints/BP_GameInstance.GI_ActivityStartDate` (struct) _asbp_game_instance)
  (`self.HandleActivityReward` (`self.ActivityCurrent`))
  (set `self.ActivityCurrent` (struct))
  (`KismetSystemLibrary.K2_ClearAndInvalidateTimerHandle` (`self.ActivityTimer`))
  (set `self.ActivityTimer` (struct)))

(fn `Skip Activity`
  (if (`KismetSystemLibrary.K2_IsValidTimerHandle` (`self.ActivityTimer`))
    (`KismetSystemLibrary.K2_ClearAndInvalidateTimerHandle` (`self.ActivityTimer`))
    (`self.HandleActivityReward` (`self.ActivityCurrent`) true)
    (bind _asbp_game_instance (`/Game/Blueprints/FunctionLibraries/FL_GameInstance.GetGameInstance`))
    (set `/Game/Blueprints/BP_GameInstance.GI_ActivityCurrent` (struct) _asbp_game_instance)
    (set `/Game/Blueprints/BP_GameInstance.GI_ActivityStartDate` (struct) _asbp_game_instance)
    (set `self.ActivityCurrent` (struct))
    (set `self.ActivityTimer` (struct))))

(fn `Start Activity`
  (params (Activity :type "/Game/Blueprints/Structs/S_Activity Structure (by ref)"))
  (bind (_id _name _uses _stats _availabletime _availabledays _timetocomplete) (break `/Game/Blueprints/Structs/S_Activity` Activity))
  (bind _activityusages (`self.ActivityUsages`))
  (bind _activityusages_2 (`self.ActivityUsages`))
  (bind _asbp_game_instance (`/Game/Blueprints/FunctionLibraries/FL_GameInstance.GetGameInstance`))
  (set `/Game/Blueprints/BP_GameInstance.GI_ActivityCurrent` Activity _asbp_game_instance)
  (bind _continue (`self.Start Special Activity` Activity))
  (if _continue
    (`self.OnActivityStarted`)
    (bind _returnvalue (`KismetSystemLibrary.K2_SetTimerDelegate` (`|CreateDelegate` :!event `OnFinishActivityTimer`) _timetocomplete))
    (set `self.ActivityTimer` _returnvalue)
    (set `/Game/Blueprints/BP_GameInstance.GI_ActivityStartDate` (`KismetMathLibrary.Now`) _asbp_game_instance)
    (if (`BlueprintMapLibrary.Map_Contains` _activityusages _id)
      (`BlueprintMapLibrary.Map_Add` _activityusages_2 _id (+ (`BlueprintMapLibrary.Map_Find` _activityusages _id) 1))
      (else
        (`BlueprintMapLibrary.Map_Add` _activityusages_2 _id 2)))
    (bind _asbp_game_instance_2 (`/Game/Blueprints/FunctionLibraries/FL_GameInstance.GetGameInstance`))
    (set `/Game/Blueprints/BP_GameInstance.GI_ActivityUsages` (`self.ActivityUsages`) _asbp_game_instance_2)))

(fn `Start Special Activity`
  (params (Activity :type "/Game/Blueprints/Structs/S_Activity Structure (by ref)"))
  (returns (Continue :type Boolean))
  (locals (ShouldContinue :type Boolean))
  (bind (_id _name _uses _stats _availabletime _availabledays _timetocomplete _activitytype) (break `/Game/Blueprints/Structs/S_Activity` Activity))
  (set `local.ShouldContinue` false)
  (switch `/Game/Blueprints/Enums/E_ActivityType` _activitytype
    (:`NewEnumerator0`
      (set `local.ShouldContinue` true)
      (return (`local.ShouldContinue`)))
    (:`NewEnumerator1`
      (switch `int` _id
        (:`200`
          (set `local.ShouldContinue` true :!label _label)
          (return (`local.ShouldContinue`)))
        (:`201`
          (goto _label))
        (:`202`
          (bind (_isvalid _stagemanager) (`/Game/Blueprints/FunctionLibraries/FL_GameInstance.GetStageManager`))
          (if _isvalid
            (if (`/Game/Blueprints/Managers/BP_StageManager.StudentCanStudy` _stagemanager)
              (goto _label)
              (else
                (return (`local.ShouldContinue`))))))
        (:`203`
          (bind (_isvalid_2 _stagemanager_2) (`/Game/Blueprints/FunctionLibraries/FL_GameInstance.GetStageManager`))
          (if _isvalid_2
            (if (`/Game/Blueprints/Managers/BP_StageManager.WorkerCanWork` _stagemanager_2)
              (goto _label)
              (else
                (return (`local.ShouldContinue`))))))))))

(fn `UserConstructionScript`)