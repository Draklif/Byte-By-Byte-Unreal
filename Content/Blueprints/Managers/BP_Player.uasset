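; Player manager for a life-sim, owning the player's stats, money, job and inventory.
; BeginPlay copies state from the GameInstance, and mutators write changes back to persist it.
; Using an item applies its stat changes, consumes one and counts toward a daily limit, cleared on the WorldManager's new-day event.
; Stat changes are clamped, work pay and study gains derive from job, knowledge or stress values, and high hunger-stat values can add weight.
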(event `Reset Sleep`)

(event `self.ReceiveBeginPlay`
  (bind _asbp_game_instance (`/Game/Blueprints/FunctionLibraries/FL_GameInstance.GetGameInstance`))
  (set `self.PlayerStats` (`/Game/Blueprints/BP_GameInstance.GI_PlayerStats` _asbp_game_instance))
  (set `self.PlayerInventory` (`/Game/Blueprints/BP_GameInstance.GI_PlayerInventory` _asbp_game_instance))
  (set `self.ItemUsages` (`/Game/Blueprints/BP_GameInstance.GI_ItemUsages` _asbp_game_instance))
  (bind (_isvalid _worldmanager) (`/Game/Blueprints/FunctionLibraries/FL_GameInstance.GetWorldManager`))
  (add `/Game/Blueprints/Managers/BP_WorldManager.OnNewDay` _worldmanager (delegate `Reset Item Usages`))
  (add `/Game/Blueprints/Managers/BP_WorldManager.OnNewDay` _worldmanager (delegate `Reset Sleep`)))

(event `Reset Item Usages`
  (`BlueprintMapLibrary.Map_Clear` (`self.ItemUsages`))
  (bind _asbp_game_instance (`/Game/Blueprints/FunctionLibraries/FL_GameInstance.GetGameInstance`))
  (set `/Game/Blueprints/BP_GameInstance.GI_ItemUsages` (`self.ItemUsages`) _asbp_game_instance))

(fn `AddHappiness`
  (params (Value :type Integer))
  (bind _playerstats (`self.PlayerStats`))
  (bind _structout (setmembers `/Game/Blueprints/Structs/S_PlayerStats` :`StructRef` _playerstats :`Happiness` (`KismetMathLibrary.Clamp` (+ (`.Happiness_4_9F24056243AAD87582BE5DB703BD4DA3` (break `/Game/Blueprints/Structs/S_PlayerStats` _playerstats)) Value) 0 100)))
  (bind _output_get (set `self.PlayerStats` _structout))
  (bind _asbp_game_instance (`/Game/Blueprints/FunctionLibraries/FL_GameInstance.GetGameInstance`))
  (set `/Game/Blueprints/BP_GameInstance.GI_PlayerStats` _output_get _asbp_game_instance))

(fn `AddHunger`
  (params (Value :type Integer))
  (bind _playerstats (`self.PlayerStats`))
  (bind _structout (setmembers `/Game/Blueprints/Structs/S_PlayerStats` :`StructRef` _playerstats :`Hunger` (`KismetMathLibrary.Clamp` (+ (`.Hunger_5_8E3AEE664DA003FE5FB31ABD561EEAB5` (break `/Game/Blueprints/Structs/S_PlayerStats` _playerstats)) Value) 0 100)))
  (bind _output_get (set `self.PlayerStats` _structout))
  (bind _asbp_game_instance (`/Game/Blueprints/FunctionLibraries/FL_GameInstance.GetGameInstance`))
  (set `/Game/Blueprints/BP_GameInstance.GI_PlayerStats` _output_get _asbp_game_instance))

(fn `AddItem`
  (params (Item :type "/Game/Blueprints/Structs/S_Item Structure"))
  (locals (ItemToAdd :type "/Game/Blueprints/Structs/S_Item Structure") (HasFoundItem :type Boolean))
  (bind _itemtoadd (`local.ItemToAdd`))
  (bind _playerinventory (`self.PlayerInventory`))
  (bind _playerinventory_2 (`self.PlayerInventory`))
  (bind _structout (setmembers `/Game/Blueprints/Structs/S_Item` :`StructRef` Item :`Quantity` 1))
  (set `local.ItemToAdd` _structout)
  (for _array_element _playerinventory
    (bind (_id _name _description _uses _quantity) (break `/Game/Blueprints/Structs/S_Item` _array_element))
    (if (== _id (`.Id_38_BD91578A4EDE77757E6282847788F1A4` (break `/Game/Blueprints/Structs/S_Item` _itemtoadd)))
      (set `local.HasFoundItem` true)
      (bind _structout_2 (setmembers `/Game/Blueprints/Structs/S_Item` :`StructRef` _array_element :`Quantity` (+ _quantity 1)))
      (`KismetArrayLibrary.Array_RemoveItem` _playerinventory _array_element)
      (`KismetArrayLibrary.Array_Add` _playerinventory _structout_2)))
  (if (not (`local.HasFoundItem`))
    (`KismetArrayLibrary.Array_Add` _playerinventory_2 _itemtoadd))
  (bind _asbp_game_instance (`/Game/Blueprints/FunctionLibraries/FL_GameInstance.GetGameInstance`))
  (set `/Game/Blueprints/BP_GameInstance.GI_PlayerInventory` _playerinventory_2 _asbp_game_instance))

(fn `AddKnowledge`
  (params (Value :type Integer))
  (bind _playerstats (`self.PlayerStats`))
  (bind _structout (setmembers `/Game/Blueprints/Structs/S_PlayerStats` :`StructRef` _playerstats :`Knowledge` (`KismetMathLibrary.Clamp` (+ (`.Knowledge_11_4E54FEA9483A9DA9B3A737BFA2887292` (break `/Game/Blueprints/Structs/S_PlayerStats` _playerstats)) Value) 0 100)))
  (bind _output_get (set `self.PlayerStats` _structout))
  (bind _asbp_game_instance (`/Game/Blueprints/FunctionLibraries/FL_GameInstance.GetGameInstance`))
  (set `/Game/Blueprints/BP_GameInstance.GI_PlayerStats` _output_get _asbp_game_instance))

(fn `AddMoney`
  (params (Money :type Integer))
  (bind _playerstats (`self.PlayerStats`))
  (bind _structout (setmembers `/Game/Blueprints/Structs/S_PlayerStats` :`StructRef` _playerstats :`Money` (+ (`.Money_13_52FBA7074E5A81AD30E96292D47CF16D` (break `/Game/Blueprints/Structs/S_PlayerStats` _playerstats)) Money)))
  (bind _output_get (set `self.PlayerStats` _structout))
  (bind _asbp_game_instance (`/Game/Blueprints/FunctionLibraries/FL_GameInstance.GetGameInstance`))
  (set `/Game/Blueprints/BP_GameInstance.GI_PlayerStats` _output_get _asbp_game_instance))

(fn `AddPosition`
  (params (AddPosition :type "Float (double-precision)"))
  (bind _playerstats (`self.PlayerStats`))
  (bind _structout (setmembers `/Game/Blueprints/Structs/S_PlayerStats` :`StructRef` _playerstats :`PositionMult` (+ (`KismetMathLibrary.FClamp` (`.PositionMult_18_69BB09F7402E2769A01892944B67D727` (break `/Game/Blueprints/Structs/S_PlayerStats` _playerstats)) 1.0 6.0) AddPosition)))
  (bind _output_get (set `self.PlayerStats` _structout))
  (bind _asbp_game_instance (`/Game/Blueprints/FunctionLibraries/FL_GameInstance.GetGameInstance`))
  (set `/Game/Blueprints/BP_GameInstance.GI_PlayerStats` _output_get _asbp_game_instance))

(fn `AddSalary`
  (params (BaseSalary :type "Float (double-precision)"))
  (bind _playerstats (`self.PlayerStats`))
  (bind (_stage _happiness _hunger _stress _weight _knowledge _money _basesalary) (break `/Game/Blueprints/Structs/S_PlayerStats` _playerstats))
  (bind _structout (setmembers `/Game/Blueprints/Structs/S_PlayerStats` :`StructRef` _playerstats :`BaseSalary` (+ (* _basesalary BaseSalary) _basesalary)))
  (bind _output_get (set `self.PlayerStats` _structout))
  (bind _asbp_game_instance (`/Game/Blueprints/FunctionLibraries/FL_GameInstance.GetGameInstance`))
  (set `/Game/Blueprints/BP_GameInstance.GI_PlayerStats` _output_get _asbp_game_instance))

(fn `AddStress`
  (params (Value :type Integer))
  (bind _playerstats (`self.PlayerStats`))
  (bind _structout (setmembers `/Game/Blueprints/Structs/S_PlayerStats` :`StructRef` _playerstats :`Stress` (`KismetMathLibrary.Clamp` (+ (`.Stress_7_416411EE49C372E6C366F5ADDC3FC9CA` (break `/Game/Blueprints/Structs/S_PlayerStats` _playerstats)) Value) 0 100)))
  (bind _output_get (set `self.PlayerStats` _structout))
  (bind _asbp_game_instance (`/Game/Blueprints/FunctionLibraries/FL_GameInstance.GetGameInstance`))
  (set `/Game/Blueprints/BP_GameInstance.GI_PlayerStats` _output_get _asbp_game_instance))

(fn `AddWeight`
  (params (Value :type Integer))
  (bind _playerstats (`self.PlayerStats`))
  (bind _structout (setmembers `/Game/Blueprints/Structs/S_PlayerStats` :`StructRef` _playerstats :`Weight` (`KismetMathLibrary.Clamp` (+ (`.Weight_9_675F643543BDC9FCC0D059A00F05BB82` (break `/Game/Blueprints/Structs/S_PlayerStats` _playerstats)) Value) 0 100)))
  (bind _output_get (set `self.PlayerStats` _structout))
  (bind _asbp_game_instance (`/Game/Blueprints/FunctionLibraries/FL_GameInstance.GetGameInstance`))
  (set `/Game/Blueprints/BP_GameInstance.GI_PlayerStats` _output_get _asbp_game_instance))

(fn `GetMoney`
  (returns (Money :type Integer))
  (return (`.Money_13_52FBA7074E5A81AD30E96292D47CF16D` (break `/Game/Blueprints/Structs/S_PlayerStats` (`self.PlayerStats`)))))

(fn `ModifyKnowledgeStudy`
  (params (Time :type Integer) (Halved :type Boolean))
  (bind (_stage _happiness _hunger _stress _weight _knowledge _money _basesalary _positionmult _knowledgemult) (break `/Game/Blueprints/Structs/S_PlayerStats` (`self.PlayerStats`)))
  (bind _returnvalue (`KismetMathLibrary.FTrunc` (* _knowledgemult 10.0 Time (- 1.0 (/ _stress 100)))))
  (if Halved
    (`self.AddKnowledge` (/ _returnvalue 2))
    (else
      (`self.AddKnowledge` _returnvalue)))
  (`self.AddStress` (* 10 (- Time 1)))
  (`self.AddHunger` (* _returnvalue -1)))

(fn `ModifyMoneyWork`
  (params (Halved :type Boolean))
  (locals (Money :type "Float (double-precision)"))
  (bind (_stage _happiness _hunger _stress _weight _knowledge _money _basesalary _positionmult _knowledgemult) (break `/Game/Blueprints/Structs/S_PlayerStats` (`self.PlayerStats`)))
  (set `local.Money` (* (+ (* _basesalary _positionmult) (* _knowledge _knowledgemult)) (`KismetMathLibrary.RandomFloatInRange` 0.8 1.2)))
  (if Halved
    (set `local.Money` (/ (`local.Money`) 2.0)))
  (`self.AddMoney` (`KismetMathLibrary.FTrunc` (`local.Money`))))

(fn `ModifyPlayerStats`
  (params (StatsValues :type "Array of /Game/Blueprints/Structs/S_StatValue Structure") (Halved :type Boolean))
  (locals (Value :type Integer))
  (for _array_element StatsValues
    (`self.ModifyStat` _array_element Halved)))

(fn `ModifyStat`
  (params (`Stat Value` :type "/Game/Blueprints/Structs/S_StatValue Structure (by ref)") (Halved :type Boolean))
  (locals (Value :type Integer))
  (bind (_stat _value) (break `/Game/Blueprints/Structs/S_StatValue` `Stat Value`))
  (bind _value_2 (`local.Value`))
  (set `local.Value` _value)
  (if Halved
    (set `local.Value` (/ (`local.Value`) 2)))
  (switch `/Game/Blueprints/Enums/E_Stat` _stat
    (:`NewEnumerator0`
      (`self.AddHappiness` _value_2))
    (:`NewEnumerator1`
      (if (>= (`.Hunger_5_8E3AEE664DA003FE5FB31ABD561EEAB5` (break `/Game/Blueprints/Structs/S_PlayerStats` (`self.PlayerStats`))) 80)
        (`self.AddWeight` (`KismetMathLibrary.FFloor` (`KismetMathLibrary.FClamp` (* 10.0 (`KismetMathLibrary.MultiplyMultiply_FloatFloat` (`KismetMathLibrary.Conv_IntToDouble` (/ (`local.Value`) 70)) 2.0)) 0.5 10.0))))
      (`self.AddHunger` (`local.Value`)))
    (:`NewEnumerator2`
      (`self.AddStress` _value_2))
    (:`NewEnumerator3`
      (`self.AddWeight` _value_2))
    (:`NewEnumerator4`
      (`self.AddKnowledge` _value_2))))

(fn `RemoveItem`
  (params (Item :type "/Game/Blueprints/Structs/S_Item Structure (by ref)"))
  (locals (ItemToRemove :type "/Game/Blueprints/Structs/S_Item Structure"))
  (bind _playerinventory (`self.PlayerInventory`))
  (bind _returnvalue (`KismetArrayLibrary.Array_Find` _playerinventory Item))
  (bind _output (`|GetArrayItem` _playerinventory _returnvalue))
  ;[1 1 1] Check if Item Exists in Player Inventory
  (if (> _returnvalue -1)
    ;[1 1 1] Decreace and/or remove item in inventory
    (bind _output_get (set `local.ItemToRemove` _output))
    (bind _result (`/Engine/EditorBlueprintResources/StandardMacros.DecrementInt` (`.Quantity_20_891038D2415BFF5507C749AB8C7AEA4C` (break `/Game/Blueprints/Structs/S_Item` _output_get)))
      (:`  `
        (if (> _result 0)
          (`KismetArrayLibrary.Array_Set` _playerinventory _returnvalue (`local.ItemToRemove`))
          (else
            (`KismetArrayLibrary.Array_RemoveItem` _playerinventory _output)))
        (`self.OnInventoryUpdated`)
        (bind _asbp_game_instance (`/Game/Blueprints/FunctionLibraries/FL_GameInstance.GetGameInstance`))
        (set `/Game/Blueprints/BP_GameInstance.GI_PlayerInventory` (`self.PlayerInventory`) _asbp_game_instance)))))

(fn `SetJob`
  (params (BaseSalary :type "Float (double-precision)") (KnowledgeMult :type "Float (double-precision)") (StressMult :type "Float (double-precision)"))
  (bind _structout (setmembers `/Game/Blueprints/Structs/S_PlayerStats` :`StructRef` (`self.PlayerStats`) :`BaseSalary` BaseSalary :`KnowledgeMult` KnowledgeMult :`StressMult` StressMult))
  (bind _output_get (set `self.PlayerStats` _structout))
  (bind _asbp_game_instance (`/Game/Blueprints/FunctionLibraries/FL_GameInstance.GetGameInstance`))
  (set `/Game/Blueprints/BP_GameInstance.GI_PlayerStats` _output_get _asbp_game_instance))

(fn `SetPosition`
  (params (PositionMult :type "Float (double-precision)"))
  (bind _structout (setmembers `/Game/Blueprints/Structs/S_PlayerStats` :`StructRef` (`self.PlayerStats`) :`PositionMult` PositionMult))
  (bind _output_get (set `self.PlayerStats` _structout))
  (bind _asbp_game_instance (`/Game/Blueprints/FunctionLibraries/FL_GameInstance.GetGameInstance`))
  (set `/Game/Blueprints/BP_GameInstance.GI_PlayerStats` _output_get _asbp_game_instance))

(fn `SetStage`
  (params (Stage :type "/Game/Blueprints/Enums/E_PlayerStage Enum" :default "NewEnumerator0"))
  (bind _structout (setmembers `/Game/Blueprints/Structs/S_PlayerStats` :`StructRef` (`self.PlayerStats`) :`Stage` Stage))
  (bind _output_get (set `self.PlayerStats` _structout))
  (bind _asbp_game_instance (`/Game/Blueprints/FunctionLibraries/FL_GameInstance.GetGameInstance`))
  (set `/Game/Blueprints/BP_GameInstance.GI_PlayerStats` _output_get _asbp_game_instance))

(fn `UseItem`
  (params (Item :type "/Game/Blueprints/Structs/S_Item Structure (by ref)"))
  (bind (_id _name _description _uses _quantity _price _rarity _stats) (break `/Game/Blueprints/Structs/S_Item` Item))
  (bind _itemusages (`self.ItemUsages`))
  (bind _itemusages_2 (`self.ItemUsages`))
  (bind _returnvalue (`BlueprintMapLibrary.Map_Contains` _itemusages _id))
  (bind _value (`BlueprintMapLibrary.Map_Find` _itemusages _id))
  ;[1 1 1] Check if Item Exists in Player Inventory
  (if (> (`KismetArrayLibrary.Array_Find` (`self.PlayerInventory`) Item) -1)
    (if (and _returnvalue (>= _value _uses))
      (`/Game/Blueprints/FunctionLibraries/FL_Utilities.PlayTip` "No more uses" "No more uses remaining for this item today." 3.0)
      (else
        (if _returnvalue
          (`BlueprintMapLibrary.Map_Add` _itemusages_2 _id (+ _value 1))
          (else
            (`BlueprintMapLibrary.Map_Add` _itemusages_2 _id 1)))
        (`self.ModifyPlayerStats` _stats)
        (`self.RemoveItem` Item)
        (bind _asbp_game_instance (`/Game/Blueprints/FunctionLibraries/FL_GameInstance.GetGameInstance`))
        (set `/Game/Blueprints/BP_GameInstance.GI_ItemUsages` (`self.ItemUsages`) _asbp_game_instance)))))

(fn `UserConstructionScript`)