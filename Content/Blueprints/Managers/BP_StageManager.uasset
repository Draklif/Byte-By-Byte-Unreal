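; Stage manager that runs the player's student and worker career stages in a life-sim game.
; Study and work actions use Knowledge to drive GPA, exams and deadlines, with state mirrored to the GameInstance.
; WorldManager day and week events refresh action flags, adjust GPA by attendance and roll deadline-based promotions, raises, demotions or job loss.
; Finishing the student stage offers jobs from DT_Jobs filtered by GPA.
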(event `CalculateDealines`
  (bind _workerdeadlinethreshold (`self.WorkerDeadlineThreshold`))
  (bind _workerdeadlines (`self.WorkerDeadlines`))
  (bind (_isvalid _player) (`/Game/Blueprints/FunctionLibraries/FL_GameInstance.GetPlayer`))
  (if _isvalid
    (switch `int` (`KismetMathLibrary.FTrunc` (`.PositionMult_18_69BB09F7402E2769A01892944B67D727` (break `/Game/Blueprints/Structs/S_PlayerStats` (`/Game/Blueprints/Managers/BP_Player.PlayerStats` _player))))
      (:`1`
        (set `self.WorkerDeadlineThreshold` 5))
      (:`2`
        (set `self.WorkerDeadlineThreshold` 5))
      (:`3`
        (set `self.WorkerDeadlineThreshold` 4))
      (:`4`
        (set `self.WorkerDeadlineThreshold` 4))
      (:`5`
        (set `self.WorkerDeadlineThreshold` 3))
      (:`6`
        (set `self.WorkerDeadlineThreshold` 2)))
    (if (>= _workerdeadlines _workerdeadlinethreshold)
      (set `self.WorkerDeadlineScore` "NewEnumerator0")
      (`self.CalculateWorkBonus` (`self.WorkerDeadlineScore`) :!label _label)
      (elif (>= _workerdeadlines (- _workerdeadlinethreshold 2))
        (set `self.WorkerDeadlineScore` "NewEnumerator1")
        (goto _label)
        (elif (>= _workerdeadlines (- _workerdeadlinethreshold 4))
          (set `self.WorkerDeadlineScore` "NewEnumerator4")
          (goto _label)
          (elif (>= _workerdeadlines (- _workerdeadlinethreshold 5))
            (set `self.WorkerDeadlineScore` "NewEnumerator5")
            (goto _label)))))))

(event `self.ReceiveBeginPlay`
  (bind _asbp_game_instance (`/Game/Blueprints/FunctionLibraries/FL_GameInstance.GetGameInstance`))
  (`|ExecutionSequence`
    (:`then_0`
      (set `self.StudentGPA` (`/Game/Blueprints/BP_GameInstance.GI_Student_GPA` _asbp_game_instance))
      (set `self.StudentAssistance` (`/Game/Blueprints/BP_GameInstance.GI_Student_Assistance` _asbp_game_instance))
      (set `self.StudentCanStudy` (`/Game/Blueprints/BP_GameInstance.GI_Student_CanStudy` _asbp_game_instance)))
    (:`then_1`
      (set `self.WorkerDeadlines` (`/Game/Blueprints/BP_GameInstance.GI_Worker_Deadlines` _asbp_game_instance))
      (set `self.WorkerCanWork` (`/Game/Blueprints/BP_GameInstance.GI_Worker_CanWork` _asbp_game_instance)))
    (:`then_2`
      (bind (_isvalid _worldmanager) (`/Game/Blueprints/FunctionLibraries/FL_GameInstance.GetWorldManager`))
      (add `/Game/Blueprints/Managers/BP_WorldManager.OnNewDay` _worldmanager (delegate `CalculateStudy`))
      (add `/Game/Blueprints/Managers/BP_WorldManager.OnNewWeek` _worldmanager (delegate `CalculateAssistance`))
      (add `/Game/Blueprints/Managers/BP_WorldManager.OnNewWeek` _worldmanager (delegate `CalculateDealines`)))))

(event `CalculateAssistance`
  (`self.ModifyGPA` (* -5 (- 5 (`self.StudentAssistance`))))
  (`self.ModifyGPA` (* 2 (`self.StudentAssistance`)))
  (`self.ResetAssistance`))

(event `CalculateStudy`
  (bind (_isvalid _worldmanager) (`/Game/Blueprints/FunctionLibraries/FL_GameInstance.GetWorldManager`))
  (bind _dayofweek (`/Game/Blueprints/Managers/BP_WorldManager.DayOfWeek` _worldmanager))
  (if (or (`|EnumInequality` _dayofweek "NewEnumerator5") (`|EnumInequality` _dayofweek "NewEnumerator6"))
    (set `self.StudentCanStudy` true)
    (set `self.WorkerCanWork` true)
    (else
      (set `self.StudentCanStudy` false)
      (set `self.WorkerCanWork` false)))
  (bind _asbp_game_instance (`/Game/Blueprints/FunctionLibraries/FL_GameInstance.GetGameInstance`))
  (set `/Game/Blueprints/BP_GameInstance.GI_Student_CanStudy` (`self.StudentCanStudy`) _asbp_game_instance)
  (set `/Game/Blueprints/BP_GameInstance.GI_Worker_CanWork` (`self.WorkerCanWork`) _asbp_game_instance))

(fn `CalculateWorkBonus`
  (params (WorkerDeadlineScore :type "/Game/Blueprints/Enums/E_JobScore Enum" :default "NewEnumerator0"))
  (bind _returnvalue (`KismetMathLibrary.RandomFloatInRange` 0.0 1.0))
  (bind _returnvalue_2 (<= _returnvalue 0.25))
  (switch `/Game/Blueprints/Enums/E_JobScore` WorkerDeadlineScore
    (:`NewEnumerator0`
      (if _returnvalue_2
        (bind (_isvalid _player) (`/Game/Blueprints/FunctionLibraries/FL_GameInstance.GetPlayer`))
        (`/Game/Blueprints/Managers/BP_Player.AddPosition` _player 1.0)
        (`/Game/Blueprints/Managers/BP_Player.AddSalary` _player 0.1)))
    (:`NewEnumerator1`
      (bind (_isvalid_2 _player_2) (`/Game/Blueprints/FunctionLibraries/FL_GameInstance.GetPlayer`))
      (`/Game/Blueprints/Managers/BP_Player.AddSalary` _player_2 0.05))
    (:`NewEnumerator4`
      (if _returnvalue_2
        (bind (_isvalid_3 _player_3) (`/Game/Blueprints/FunctionLibraries/FL_GameInstance.GetPlayer`))
        (`/Game/Blueprints/Managers/BP_Player.AddPosition` _player_3 -1.0)
        (`/Game/Blueprints/Managers/BP_Player.AddSalary` _player_3 -0.1)))
    (:`NewEnumerator5`
      (if (<= _returnvalue 0.3)
        (bind (_isvalid_4 _player_4) (`/Game/Blueprints/FunctionLibraries/FL_GameInstance.GetPlayer`))
        (`/Game/Blueprints/Managers/BP_Player.SetPosition` _player_4 1.0)
        (`/Game/Blueprints/Managers/BP_Player.SetStage` _player_4 "NewEnumerator3")
        (`/Game/Blueprints/Managers/BP_Player.SetJob` _player_4 10.0 1.0 2.0)
        (bind _asbp_game_instance (`/Game/Blueprints/FunctionLibraries/FL_GameInstance.GetGameInstance`))
        (set `/Game/Blueprints/BP_GameInstance.GI_JobCurrent` (struct) _asbp_game_instance)))))

(fn `FinishStudentStage`
  (`KismetArrayLibrary.Array_Clear` (`self.WorkerJobs`))
  (bind _outrownames (`DataTableFunctionLibrary.GetDataTableRowNames` "/Game/Blueprints/Tables/DT_Jobs.DT_Jobs"))
  (for _array_element _outrownames
    (bind _returnvalue (`|GetDataTableRow` "/Game/Blueprints/Tables/DT_Jobs.DT_Jobs" _array_element)
      (:`then`
        (if (>= (`self.StudentGPA`) (`.GradeThreshold_23_34E54A4540E0E50AD4127E806794C4CD` (break `/Game/Blueprints/Structs/S_Job` _returnvalue)))
          (`KismetArrayLibrary.Array_Add` (`self.WorkerJobs`) _returnvalue)))))
  (bind _returnvalue_2 (`|CreateWidget` "/Game/Blueprints/UI/WBP_SelectionPopup_Job.WBP_SelectionPopup_Job_C" null (`self.WorkerJobs`) "Jobs to apply"))
  (`UserWidget.AddToViewport` _returnvalue_2 0))

(fn `GoStudy`
  (locals (PlayerKnowledge :type Integer) (ApprovalChance :type "Float (double-precision)" :default 0.4) (ActualChance :type "Float (double-precision)" :default 0.0) (DayOfWeek :type "/Game/Blueprints/Enums/E_DayOfWeek Enum" :default "NewEnumerator0"))
  (bind (_isvalid _worldmanager) (`/Game/Blueprints/FunctionLibraries/FL_GameInstance.GetWorldManager`))
  (bind _dayofweek (`/Game/Blueprints/Managers/BP_WorldManager.DayOfWeek` _worldmanager))
  (set `local.DayOfWeek` _dayofweek)
  (if (and (or (`|EnumInequality` _dayofweek "NewEnumerator5") (`|EnumInequality` _dayofweek "NewEnumerator6")) (`self.StudentCanStudy`))
    (`self.IncrementAssistance`)
    (bind (_isvalid_2 _player) (`/Game/Blueprints/FunctionLibraries/FL_GameInstance.GetPlayer`))
    (set `local.PlayerKnowledge` (`.Knowledge_11_4E54FEA9483A9DA9B3A737BFA2887292` (break `/Game/Blueprints/Structs/S_PlayerStats` (`/Game/Blueprints/Managers/BP_Player.PlayerStats` _player))))
    (if (`|EnumEquality` (`local.DayOfWeek`) "NewEnumerator4")
      (set `local.ActualChance` (`KismetMathLibrary.RandomFloatInRange` 0.0 1.0))
      (if (>= (`local.PlayerKnowledge`) 60)
        (set `local.ApprovalChance` (+ (* 0.009 (- (`local.PlayerKnowledge`) 60)) 0.6))
        (else
          (set `local.ApprovalChance` (- 0.4 (* 0.005 (- 60 (`local.PlayerKnowledge`)))))))
      (if (<= (`local.ActualChance`) (`local.ApprovalChance`))
        (`self.ModifyGPA` 10)
        (bind (_isvalid_3 _player_2) (`/Game/Blueprints/FunctionLibraries/FL_GameInstance.GetPlayer`))
        (if _isvalid_3
          (`/Game/Blueprints/Managers/BP_Player.ModifyPlayerStats` _player_2 (`|MakeArray` (make `/Game/Blueprints/Structs/S_StatValue` "NewEnumerator0" 15) (make `/Game/Blueprints/Structs/S_StatValue` "NewEnumerator2" -10)) false)
          (`/Game/Blueprints/FunctionLibraries/FL_Utilities.PlayTip` "¡Yay!" "You passed the exam. Congratulations." 5.0))
        (else
          (`self.ModifyGPA` -10)
          (bind _isvalid_4 (`/Game/Blueprints/FunctionLibraries/FL_GameInstance.GetPlayer`))
          (if _isvalid_4
            (`/Game/Blueprints/Managers/BP_Player.ModifyPlayerStats` _player_2 (`|MakeArray` (make `/Game/Blueprints/Structs/S_StatValue` "NewEnumerator0" -10) (make `/Game/Blueprints/Structs/S_StatValue` "NewEnumerator2" 15)) false)
            (`/Game/Blueprints/FunctionLibraries/FL_Utilities.PlayTip` "¡Oops!" "You failed the exam. Better luck next time." 5.0))))
      (else
        (bind (_isvalid_5 _player_3) (`/Game/Blueprints/FunctionLibraries/FL_GameInstance.GetPlayer`))
        (if _isvalid_5
          (if (>= (`.Knowledge_11_4E54FEA9483A9DA9B3A737BFA2887292` (break `/Game/Blueprints/Structs/S_PlayerStats` (`/Game/Blueprints/Managers/BP_Player.PlayerStats` _player_3))) 30)
            (`self.ModifyGPA` 2)
            (else
              (`/Game/Blueprints/FunctionLibraries/FL_Utilities.PlayTip` "¡Oops!" "Not the best day at university. You gained no GPA points." 5.0)))
          (`/Game/Blueprints/Managers/BP_Player.ModifyPlayerStats` _player_3 (`|MakeArray` (make `/Game/Blueprints/Structs/S_StatValue` "NewEnumerator4" -5) (make `/Game/Blueprints/Structs/S_StatValue` "NewEnumerator2" -10)) false)
          (bind _output_get (set `self.StudentCanStudy` false))
          (bind _asbp_game_instance (`/Game/Blueprints/FunctionLibraries/FL_GameInstance.GetGameInstance`))
          (set `/Game/Blueprints/BP_GameInstance.GI_Student_CanStudy` _output_get _asbp_game_instance))))))

(fn `GoWork`
  (locals (PlayerKnowledge :type Integer) (ApprovalChance :type "Float (double-precision)" :default 0.4) (ActualChance :type "Float (double-precision)" :default 0.0) (DayOfWeek :type "/Game/Blueprints/Enums/E_DayOfWeek Enum" :default "NewEnumerator0"))
  (bind (_isvalid _worldmanager) (`/Game/Blueprints/FunctionLibraries/FL_GameInstance.GetWorldManager`))
  (bind _dayofweek (`/Game/Blueprints/Managers/BP_WorldManager.DayOfWeek` _worldmanager))
  (set `local.DayOfWeek` _dayofweek)
  (if (and (or (`|EnumInequality` _dayofweek "NewEnumerator5") (`|EnumInequality` _dayofweek "NewEnumerator6")) (`self.WorkerCanWork`))
    (bind (_isvalid_2 _player) (`/Game/Blueprints/FunctionLibraries/FL_GameInstance.GetPlayer`))
    (set `local.PlayerKnowledge` (`.Knowledge_11_4E54FEA9483A9DA9B3A737BFA2887292` (break `/Game/Blueprints/Structs/S_PlayerStats` (`/Game/Blueprints/Managers/BP_Player.PlayerStats` _player))))
    (bind (_isvalid_3 _player_2) (`/Game/Blueprints/FunctionLibraries/FL_GameInstance.GetPlayer`))
    (if _isvalid_3
      (if (>= (`.Knowledge_11_4E54FEA9483A9DA9B3A737BFA2887292` (break `/Game/Blueprints/Structs/S_PlayerStats` (`/Game/Blueprints/Managers/BP_Player.PlayerStats` _player_2))) (+ 50 (`KismetMathLibrary.RandomIntegerInRange` 0 20)))
        (`self.IncrementDeadlines`)
        (else
          (`/Game/Blueprints/FunctionLibraries/FL_Utilities.PlayTip` "¡Oops!" "Not the best day at work. You didn't meet the quota for the day." 5.0)))
      (`/Game/Blueprints/Managers/BP_Player.ModifyPlayerStats` _player_2 (`|MakeArray` (make `/Game/Blueprints/Structs/S_StatValue` "NewEnumerator4" -10) (make `/Game/Blueprints/Structs/S_StatValue` "NewEnumerator2" 20)) false)
      (`/Game/Blueprints/Managers/BP_Player.ModifyMoneyWork` _player_2 false)
      (bind _output_get (set `self.WorkerCanWork` false))
      (bind _asbp_game_instance (`/Game/Blueprints/FunctionLibraries/FL_GameInstance.GetGameInstance`))
      (set `/Game/Blueprints/BP_GameInstance.GI_Worker_CanWork` _output_get _asbp_game_instance))))

(fn `IncrementAssistance`
  (bind _output_get (set `self.StudentAssistance` (+ (`self.StudentAssistance`) 1)))
  (bind _asbp_game_instance (`/Game/Blueprints/FunctionLibraries/FL_GameInstance.GetGameInstance`))
  (set `/Game/Blueprints/BP_GameInstance.GI_Student_Assistance` _output_get _asbp_game_instance))

(fn `IncrementDeadlines`
  (bind _output_get (set `self.WorkerDeadlines` (+ (`self.WorkerDeadlines`) 1)))
  (bind _asbp_game_instance (`/Game/Blueprints/FunctionLibraries/FL_GameInstance.GetGameInstance`))
  (set `/Game/Blueprints/BP_GameInstance.GI_Worker_Deadlines` _output_get _asbp_game_instance))

(fn `ModifyGPA`
  (params (Value :type Integer))
  (bind _output_get (set `self.StudentGPA` (`KismetMathLibrary.Clamp` (+ (`self.StudentGPA`) Value) 0 50)))
  (`self.OnGPAUpdated`)
  (bind _asbp_game_instance (`/Game/Blueprints/FunctionLibraries/FL_GameInstance.GetGameInstance`))
  (set `/Game/Blueprints/BP_GameInstance.GI_Student_GPA` _output_get _asbp_game_instance))

(fn `ResetAssistance`
  (bind _output_get (set `self.StudentAssistance` 0))
  (bind _asbp_game_instance (`/Game/Blueprints/FunctionLibraries/FL_GameInstance.GetGameInstance`))
  (set `/Game/Blueprints/BP_GameInstance.GI_Student_Assistance` _output_get _asbp_game_instance))

(fn `ResetDeadlines`
  (bind _output_get (set `self.WorkerDeadlines` 0))
  (bind _asbp_game_instance (`/Game/Blueprints/FunctionLibraries/FL_GameInstance.GetGameInstance`))
  (set `/Game/Blueprints/BP_GameInstance.GI_Worker_Deadlines` _output_get _asbp_game_instance))

(fn `SelectJob`
  (params (Job :type "/Game/Blueprints/Structs/S_Job Structure"))
  (bind (_id _name _description _gradethreshold _basesalary _knowledgemult _stressimpact) (break `/Game/Blueprints/Structs/S_Job` Job))
  (bind (_isvalid _player) (`/Game/Blueprints/FunctionLibraries/FL_GameInstance.GetPlayer`))
  (if _isvalid
    (`/Game/Blueprints/Managers/BP_Player.SetJob` _player _basesalary _knowledgemult _stressimpact)
    (`/Game/Blueprints/Managers/BP_Player.SetStage` _player "NewEnumerator1")
    (bind _asbp_game_instance (`/Game/Blueprints/FunctionLibraries/FL_GameInstance.GetGameInstance`))
    (set `/Game/Blueprints/BP_GameInstance.GI_JobCurrent` Job _asbp_game_instance)))

(fn `UserConstructionScript`)