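; Shop manager that stocks a random item shop each new day and handles player purchases.
; Restocking rerolls random items through rarity and day-of-week checks until three distinct entries exist, stacking duplicates as quantity.
; Stock is cached in the GameInstance and reloaded on BeginPlay, regenerating if empty.
; BuyItem checks stock, the player's three-slot inventory and money, then transfers the item and broadcasts a shop update.
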(event `self.ReceiveBeginPlay`
  (bind (_isvalid _worldmanager) (`/Game/Blueprints/FunctionLibraries/FL_GameInstance.GetWorldManager`))
  (add `/Game/Blueprints/Managers/BP_WorldManager.OnNewDay` _worldmanager (delegate `GenerateShop`))
  (`self.LoadShop`))

(event `GenerateShop`
  (bind _shopinventory (`self.ShopInventory`))
  (`KismetArrayLibrary.Array_Clear` _shopinventory)
  (while (< (`KismetArrayLibrary.Array_Length` _shopinventory) 3)
    (bind (_found _row) (`/Game/Blueprints/FunctionLibraries/FL_Utilities.GetRandomItem` :!label _label))
    (if _found
      (bind (_isvalid _worldmanager) (`/Game/Blueprints/FunctionLibraries/FL_GameInstance.GetWorldManager`))
      (if _isvalid
        (bind _is_available (`self.CheckAvailability` _row (`/Game/Blueprints/Managers/BP_WorldManager.DayOfWeek` _worldmanager)))
        (bind _hit_rarity (`self.CheckRarity` _row))
        (if (and _hit_rarity _is_available)
          _
          (else
            (goto _label)))
        (else
          (bind _hit_rarity_2 (`self.CheckRarity` _row))
          (if _hit_rarity_2
            _
            (else
              (goto _label)))))
      (`self.AddItem` _row)))
  (bind _asbp_game_instance (`/Game/Blueprints/FunctionLibraries/FL_GameInstance.GetGameInstance`))
  (set `/Game/Blueprints/BP_GameInstance.GI_ShopInventory` (`self.ShopInventory`) _asbp_game_instance)
  (`self.OnShopUpdated`))

(event `LoadShop`
  (bind _asbp_game_instance (`/Game/Blueprints/FunctionLibraries/FL_GameInstance.GetGameInstance`))
  (bind _gi_shopinventory (`/Game/Blueprints/BP_GameInstance.GI_ShopInventory` _asbp_game_instance))
  (if (`KismetArrayLibrary.Array_IsEmpty` _gi_shopinventory)
    (`self.GenerateShop`)
    (else
      (set `self.ShopInventory` _gi_shopinventory)
      (`self.OnShopUpdated`))))

(fn `AddItem`
  (params (Item :type "/Game/Blueprints/Structs/S_Item Structure (by ref)"))
  (locals (HasFoundItem :type Boolean) (ItemToAdd :type "/Game/Blueprints/Structs/S_Item Structure"))
  (bind _shopinventory (`self.ShopInventory`))
  (bind _shopinventory_2 (`self.ShopInventory`))
  (bind _itemtoadd (`local.ItemToAdd`))
  (set `local.ItemToAdd` Item)
  (for _array_element _shopinventory_2
    (bind (_id _name _description _uses _quantity) (break `/Game/Blueprints/Structs/S_Item` _array_element))
    (if (== _id (`.Id_38_BD91578A4EDE77757E6282847788F1A4` (break `/Game/Blueprints/Structs/S_Item` _itemtoadd)))
      (set `local.HasFoundItem` true)
      (bind _structout (setmembers `/Game/Blueprints/Structs/S_Item` :`StructRef` _array_element :`Quantity` (+ _quantity 1)))
      (`KismetArrayLibrary.Array_RemoveItem` _shopinventory_2 _array_element)
      (`KismetArrayLibrary.Array_Add` _shopinventory_2 _structout)))
  (if (not (`local.HasFoundItem`))
    (`KismetArrayLibrary.Array_Add` _shopinventory _itemtoadd))
  (bind _asbp_game_instance (`/Game/Blueprints/FunctionLibraries/FL_GameInstance.GetGameInstance`))
  (set `/Game/Blueprints/BP_GameInstance.GI_ShopInventory` _shopinventory _asbp_game_instance))

(fn `BuyItem`
  (params (Item :type "/Game/Blueprints/Structs/S_Item Structure (by ref)"))
  (locals (HasFoundItem :type Boolean) (ItemToRemove :type "/Game/Blueprints/Structs/S_Item Structure"))
  (bind (_id _name _description _uses _quantity _price) (break `/Game/Blueprints/Structs/S_Item` Item))
  (bind _shopinventory (`self.ShopInventory`))
  (bind _returnvalue (`KismetArrayLibrary.Array_Find` _shopinventory Item))
  (bind _output (`|GetArrayItem` _shopinventory _returnvalue))
  ;[1 1 1] Check if Item Exists In Shop
  (if (> _returnvalue -1)
    ;[1 1 1] Check if Player has Money to Buy
    (bind (_isvalid _player) (`/Game/Blueprints/FunctionLibraries/FL_GameInstance.GetPlayer`))
    (if _isvalid
      (bind _playerinventory (`/Game/Blueprints/Managers/BP_Player.PlayerInventory` _player))
      (for _array_element _playerinventory
        (if (== (`.Id_38_BD91578A4EDE77757E6282847788F1A4` (break `/Game/Blueprints/Structs/S_Item` _array_element)) _id)
          (set `local.HasFoundItem` true)
          (break)))
      (if (or (< (`KismetArrayLibrary.Array_Length` _playerinventory) 3) (`local.HasFoundItem`))
        (bind _money (`/Game/Blueprints/Managers/BP_Player.GetMoney` _player))
        (if (>= _money _price)
          (`/Game/Blueprints/Managers/BP_Player.AddMoney` _player (* _price -1))
          ;[1 1 1] Decreace and/or remove item in shop
          (bind _output_get (set `local.ItemToRemove` _output))
          (bind _result (`/Engine/EditorBlueprintResources/StandardMacros.DecrementInt` (`.Quantity_20_891038D2415BFF5507C749AB8C7AEA4C` (break `/Game/Blueprints/Structs/S_Item` _output_get)))
            (:`  `
              (if (> _result 0)
                (`KismetArrayLibrary.Array_Set` _shopinventory _returnvalue (`local.ItemToRemove`))
                (else
                  (`KismetArrayLibrary.Array_RemoveItem` _shopinventory _output)))
              (`/Game/Blueprints/Managers/BP_Player.AddItem` _player (`local.ItemToRemove`))
              (`self.OnShopUpdated`)
              (bind _asbp_game_instance (`/Game/Blueprints/FunctionLibraries/FL_GameInstance.GetGameInstance`))
              (set `/Game/Blueprints/BP_GameInstance.GI_ShopInventory` (`self.ShopInventory`) _asbp_game_instance))))
        (else
          (`/Game/Blueprints/FunctionLibraries/FL_Utilities.PlayTip` "No space" "Can't add more items to inventory" 3.0))))))

(fn `CheckAvailability`
  (params (Item :type "/Game/Blueprints/Structs/S_Item Structure") (Day :type "/Game/Blueprints/Enums/E_DayOfWeek Enum" :default "NewEnumerator0"))
  (returns (`Is Available` :type Boolean))
  (locals (Available :type Boolean))
  (for _array_element (`.AvailableDays_30_167C65A940D48DA5A16C38B36BE38ED8` (break `/Game/Blueprints/Structs/S_Item` Item))
    (if (`|EnumEquality` _array_element Day)
      (set `local.Available` true)))
  (return (`local.Available`)))

(fn `CheckRarity`
  (params (Item :type "/Game/Blueprints/Structs/S_Item Structure"))
  (returns (`Hit Rarity` :type Boolean))
  (locals (Available :type Boolean))
  (return (<= (`KismetMathLibrary.RandomFloatInRange` 0.0 1.0) (`.Rarity_23_303F512A40F6D6888BB27AA85C00BF5B` (break `/Game/Blueprints/Structs/S_Item` Item)))))

(fn `UserConstructionScript`)