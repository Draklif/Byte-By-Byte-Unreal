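; World manager that tracks the real clock to set time of day and day of week, and signals new days, weeks and months.
; BeginPlay loads or initializes first/last-played dates in the GameInstance and plays DT_Music's track for the current time of day.
; A looping timer refreshes the clock and broadcasts time-of-day changes.
; A date-gated daily check compares played dates and elapsed time, then fires calendar dispatchers after a short delay.
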(event `Update Time`
  (bind _output_get (set `self.DateNow` (`KismetMathLibrary.Now`)))
  (`self.GetDayOfWeek`)
  (bind _time (`self.GetTimeOfDay`))
  (if (`|EnumInequality` (`self.TimeOfDay`) _time)
    (`self.OnNewTimeOfDay`))
  (set `self.TimeOfDay` _time)
  (if (!= (`.Day` (`KismetMathLibrary.BreakDateTime` _output_get)) (`KismetMathLibrary.GetDay` (`self.DateLastPlayed`)))
    (`self.CheckDaily`)))

(event `self.ReceiveBeginPlay`
  (`KismetSystemLibrary.K2_SetTimerDelegate` (delegate `Update Time`) 10.0 true true)
  (set `self.DateNow` (`KismetMathLibrary.Now`))
  (`self.SaveDateFirstPlayed`)
  (`self.SaveDateLastPlayed`)
  (bind _time (`self.GetTimeOfDay`))
  (set `self.TimeOfDay` _time)
  (`self.GetDayOfWeek`)
  (`self.GetElapsedTime`)
  (`self.CheckDaily`)
  (bind _returnvalue (`|GetDataTableRow` "/Game/Blueprints/Tables/DT_Music.DT_Music" (`KismetStringLibrary.Conv_StringToName` (`|GetEnumeratorNameAsString` (`self.TimeOfDay`))))
    (:`then`
      (`GameplayStatics.PlaySound2D` (`.Music_8_C52557EE4A4832A4D8D1C09239051DCD` (break `/Game/Blueprints/Structs/S_Music` _returnvalue)) 1.0 1.0 0.0 null null))))

(event `Call Flags`
  (`self.OnNewDay`)
  (`self.OnNewWeek`)
  (`self.OnNewMonth`))

(event `New Day`
  (`KismetSystemLibrary.Delay` 5.0)
  (`self.OnNewDay`))

(event `New Week`
  (`KismetSystemLibrary.Delay` 5.0)
  (`self.OnNewWeek`))

(event `New Month`
  (`KismetSystemLibrary.Delay` 5.0)
  (`self.OnNewMonth`))

(fn `Check Flags`
  (if (not (== (`self.DateFirstPlayed`) (`self.DateLastPlayed`)))
    (`|ExecutionSequence`
      (:`then_0`
        (if (or (>= (`KismetMathLibrary.GetDays` (`self.ElapsedTimeLastPlayed`)) 1) (!= (`KismetMathLibrary.GetDay` (`self.DateFirstPlayed`)) (`KismetMathLibrary.GetDay` (`self.DateLastPlayed`))))
          (`self.New Day`)))
      (:`then_1`
        (if (or (>= (`KismetMathLibrary.GetDays` (`self.ElapsedTimeLastPlayed`)) 7) false)
          (`self.New Week`)))
      (:`then_2`
        (if (or (>= (`KismetMathLibrary.GetDays` (`self.ElapsedTimeLastPlayed`)) 30) (!= (`KismetMathLibrary.GetMonth` (`self.DateNow`)) (`KismetMathLibrary.GetMonth` (`self.DateLastPlayed`))))
          (`self.New Month`))))))

(fn `CheckDaily`
  (locals (CanExecuteDaily :type Boolean))
  (set `local.CanExecuteDaily` true)
  (bind _asbp_game_instance (`/Game/Blueprints/FunctionLibraries/FL_GameInstance.GetGameInstance`))
  (bind _gi_datelastcheck (`/Game/Blueprints/BP_GameInstance.GI_DateLastCheck` _asbp_game_instance))
  (if (not (<= (`KismetMathLibrary.BreakDateTime` _gi_datelastcheck) 1))
    (set `self.DateLastCheck` _gi_datelastcheck)
    (set `local.CanExecuteDaily` (> (`KismetMathLibrary.GetDate` (`self.DateNow`)) (`KismetMathLibrary.GetDate` (`self.DateLastCheck`)))))
  (if (`local.CanExecuteDaily`)
    (bind _output_get (set `self.DateLastCheck` (`self.DateNow`)))
    (set `/Game/Blueprints/BP_GameInstance.GI_DateLastCheck` _output_get _asbp_game_instance)
    (`self.Check Flags`)))

(fn `GetDayOfWeek`
  (bind _returnvalue (+ (mod (`KismetMathLibrary.GetDayOfYear` (`self.DateNow`)) 7) 6))
  (set `self.DayOfWeek` (select `int` (select `bool` (> _returnvalue 6) :`false` _returnvalue :`true` (- _returnvalue 7)) :`0` "NewEnumerator0" :`1` "NewEnumerator1" :`2` "NewEnumerator2" :`3` "NewEnumerator3" :`4` "NewEnumerator4" :`5` "NewEnumerator5" :`6` "NewEnumerator6" :!type "/Game/Blueprints/Enums/E_DayOfWeek Enum")))

(fn `GetElapsedTime`
  (bind _datenow (`self.DateNow`))
  (set `self.ElapsedTimeLastPlayed` (- _datenow (`self.DateLastPlayed`)))
  (set `self.ElapsedTimeFirstPlayed` (- _datenow (`self.DateFirstPlayed`))))

(fn `GetTimeOfDay`
  (returns (Time :type "/Game/Blueprints/Enums/E_TimeOfDay Enum"))
  (bind _returnvalue (`KismetMathLibrary.GetHour` (`self.DateNow`)))
  ;[1 1 1] Morning
  (if (and (>= _returnvalue 6) (< _returnvalue 12))
    (return "NewEnumerator0")
    (else
      ;[1 1 1] Afternoon
      (if (and (>= _returnvalue 12) (< _returnvalue 18))
        (return "NewEnumerator1")
        (else
          ;[1 1 1] Evening
          (if (and (>= _returnvalue 18) (< _returnvalue 24))
            (return "NewEnumerator2")
            (else
              ;[1 1 1] Midnight
              (return "NewEnumerator3"))))))))

(fn `SaveDateFirstPlayed`
  (bind _asbp_game_instance (`/Game/Blueprints/FunctionLibraries/FL_GameInstance.GetGameInstance`))
  (bind _gi_datefirstplayed (`/Game/Blueprints/BP_GameInstance.GI_DateFirstPlayed` _asbp_game_instance))
  (if (<= (`KismetMathLibrary.BreakDateTime` _gi_datefirstplayed) 1)
    (bind _output_get (set `self.DateFirstPlayed` (`self.DateNow`)))
    (set `/Game/Blueprints/BP_GameInstance.GI_DateFirstPlayed` _output_get _asbp_game_instance)
    (else
      (bind _output_get_2 (set `self.DateFirstPlayed` _gi_datefirstplayed))
      (set `/Game/Blueprints/BP_GameInstance.GI_DateFirstPlayed` _output_get_2 _asbp_game_instance))))

(fn `SaveDateLastPlayed`
  (bind _asbp_game_instance (`/Game/Blueprints/FunctionLibraries/FL_GameInstance.GetGameInstance`))
  (bind _gi_datelastplayed (`/Game/Blueprints/BP_GameInstance.GI_DateLastPlayed` _asbp_game_instance))
  (if (<= (`KismetMathLibrary.BreakDateTime` _gi_datelastplayed) 1)
    (bind _output_get (set `self.DateLastPlayed` (`self.DateNow`)))
    (set `/Game/Blueprints/BP_GameInstance.GI_DateLastPlayed` _output_get _asbp_game_instance)
    (else
      (bind _output_get_2 (set `self.DateLastPlayed` _gi_datelastplayed))
      (set `/Game/Blueprints/BP_GameInstance.GI_DateLastPlayed` _output_get_2 _asbp_game_instance))))

(fn `UserConstructionScript`)